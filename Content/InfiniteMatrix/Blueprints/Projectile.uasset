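; Player projectile Blueprint that destroys enemies it hits and awards score.
; On BeginPlay it casts its parent actor to BP_Player and derives Speed from the player's ForwardSpeed plus an offset.
; A collision overlap with BP_Enemy destroys the enemy, adds points to the BP_Player found by class lookup, then destroys the projectile.
; The SetActorLocation step using Speed along X is disconnected, and Tick is empty.
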(event OnComponentBeginOverlap(projectilecollision)
  (params (OverlappedComponent :type Primitive%20Component%20Object%20Reference) (OtherActor :type Actor%20Object%20Reference) (OtherComp :type Primitive%20Component%20Object%20Reference) (OtherBodyIndex :type Integer) (bFromSweep :type Boolean) (SweepResult :type Hit%20Result%20Structure%20%28by%20ref%29))
  (bind _asbp_enemy (Utilities|Casting|CastToBP_Enemy OtherActor))
  (Actor|DestroyActor _asbp_enemy)
  (bind _returnvalue (Actor|GetActorOfClass "/Game/InfiniteMatrix/Blueprints/BP_Player.BP_Player_C"))
  (Variables|/Game/InfiniteMatrix/Blueprints/BP_Player.BP_Player_C|Setscore_value _returnvalue (+ (Variables|/Game/InfiniteMatrix/Blueprints/BP_Player.BP_Player_C|Getscore_value _returnvalue) 24 0))
  (Actor|DestroyActor))

(event EventBeginPlay
  (bind _asbp_player (Utilities|Casting|CastToBP_Player (Actor|GetParentActor)))
  (Variables|Default|Setspeed (+ (Variables|/Game/InfiniteMatrix/Blueprints/BP_Player.BP_Player_C|GetForwardSpeed _asbp_player) 5e+03)))

(event Collision|EventActorBeginOverlap
  (params (OtherActor :type Actor%20Object%20Reference)))

(event EventTick
  (params (DeltaSeconds :type Float%20%28single-precision%29)))

(fn ConstructionScript)